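; BP_Tiles is a shootable pair of matching tiles for a memory-style game.
; A BP_FirstPersonProjectile hit flips a cube with a timeline, recolors it and sets its flag.
; If both flags are set, MatchTile1-2 increments MatchedTiles on the BP_Lives game instance and destroys both tiles; otherwise Lives drops and the cube flips back.
; Delays and follow-up logic hang off timeline Update pins, and the W_Lose screen logic is disconnected.
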(event `self.Box1.OnComponentHit`
  (params (HitComponent :type "PrimitiveComponent Object Reference") (OtherActor :type "Actor Object Reference") (OtherComp :type "PrimitiveComponent Object Reference") (NormalImpulse :type "Vector Structure") (Hit :type "HitResult Structure (by ref)"))
  ; 1-2
  (cast `/Game/FirstPerson/Blueprints/BP_FirstPersonProjectile` OtherActor)
  (bind (_direction _newtrack_0) (`Timeline|Timeline` :!via `PlayFromStart`)
    (:`Update`
      (`SceneComponent.K2_SetRelativeRotation` (`self.Cube1`) (`KismetMathLibrary.MakeRotator` (* _newtrack_0 90.0)) false false)
      (`KismetSystemLibrary.Delay` 1.0)
      (`PrimitiveComponent.SetMaterial` (`self.Cube1`) 0 "/AnimationSharing/AnimSharingBlue.AnimSharingBlue")
      (`/Engine/EditorBlueprintResources/StandardMacros.FlipFlop`
        (:`A`
          _)
        (:`B`
          _))
      (set `self.1` true)
      (if (and (`self.1`) (`self.2`))
        (`self.MatchTile1-2`)
        (else
          (bind _asbp_lives (cast `/Game/BluePrints/BP_Lives` (`GameplayStatics.GetGameInstance`)))
          (bind _result (`/Engine/EditorBlueprintResources/StandardMacros.DecrementInt` (`/Game/BluePrints/BP_Lives.Lives` _asbp_lives))
            (:`  `
              (`KismetSystemLibrary.Delay` 1.0)
              (bind (_direction_2 _newtrack_0_2) (`Timeline|Timeline_1` :!via `PlayFromStart`)
                (:`Update`
                  (`SceneComponent.K2_SetRelativeRotation` (`self.Cube1`) (`KismetMathLibrary.MakeRotator` (* _newtrack_0_2 -90.0)) false false)
                  (`PrimitiveComponent.SetMaterial` (`self.Cube1`) 0 "/Engine/BasicShapes/BasicShapeMaterial.BasicShapeMaterial")
                  (set `self.1` false)
                  (`KismetSystemLibrary.Delay` 1.5))))))))))

(event `self.Box2.OnComponentHit`
  (params (HitComponent :type "PrimitiveComponent Object Reference") (OtherActor :type "Actor Object Reference") (OtherComp :type "PrimitiveComponent Object Reference") (NormalImpulse :type "Vector Structure") (Hit :type "HitResult Structure (by ref)"))
  ; 1-2
  (cast `/Game/FirstPerson/Blueprints/BP_FirstPersonProjectile` OtherActor)
  (bind (_direction _newtrack_0) (`Timeline|Timeline_0` :!via `PlayFromStart`)
    (:`Update`
      (`SceneComponent.K2_SetRelativeRotation` (`self.Cube2`) (`KismetMathLibrary.MakeRotator` (* _newtrack_0 90.0)) false false)
      (`KismetSystemLibrary.Delay` 1.0)
      (`PrimitiveComponent.SetMaterial` (`self.Cube2`) 0 "/AnimationSharing/AnimSharingBlue.AnimSharingBlue")
      (`/Engine/EditorBlueprintResources/StandardMacros.FlipFlop`
        (:`A`
          _)
        (:`B`
          _))
      (set `self.2` true)
      (if (and (`self.1`) (`self.2`))
        (`self.MatchTile1-2`)
        (else
          (bind _asbp_lives (cast `/Game/BluePrints/BP_Lives` (`GameplayStatics.GetGameInstance`)))
          (bind _result (`/Engine/EditorBlueprintResources/StandardMacros.DecrementInt` (`/Game/BluePrints/BP_Lives.Lives` _asbp_lives))
            (:`  `
              (`KismetSystemLibrary.Delay` 1.0)
              (bind (_direction_2 _newtrack_0_2) (`Timeline|Timeline_2` :!via `PlayFromStart`)
                (:`Update`
                  (`SceneComponent.K2_SetRelativeRotation` (`self.Cube2`) (`KismetMathLibrary.MakeRotator` (* _newtrack_0_2 -90.0)) false false)
                  (`PrimitiveComponent.SetMaterial` (`self.Cube2`) 0 "/Engine/BasicShapes/BasicShapeMaterial.BasicShapeMaterial")
                  (set `self.2` false)
                  (`KismetSystemLibrary.Delay` 1.5))))))))))

(event `MatchTile1-2`
  (if (and (`self.1`) (`self.2`))
    (`KismetSystemLibrary.Delay` 1.0)
    (bind _asbp_lives (cast `/Game/BluePrints/BP_Lives` (`GameplayStatics.GetGameInstance`)))
    (set `/Game/BluePrints/BP_Lives.MatchedTiles` (+ (`/Game/BluePrints/BP_Lives.MatchedTiles` _asbp_lives) 1) _asbp_lives)
    (`KismetSystemLibrary.Delay` 1.0)
    (`ActorComponent.K2_DestroyComponent` (`self.Box1`))
    (`ActorComponent.K2_DestroyComponent` (`self.Cube1`))
    (`ActorComponent.K2_DestroyComponent` (`self.Cube2`))
    (`ActorComponent.K2_DestroyComponent` (`self.Box2`))))

(fn `UserConstructionScript`)